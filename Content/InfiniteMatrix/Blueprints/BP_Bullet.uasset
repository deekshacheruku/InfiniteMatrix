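; BP_Bullet is a projectile actor that travels in a straight line through the world.
; SetDirection stores a Direction vector, which acts as velocity because its magnitude sets the speed.
; Tick adds Direction scaled by DeltaSeconds to the actor location, giving frame-rate independent motion without a movement component.
; The graphs contain no hit, damage or lifetime logic.
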(event EventBeginPlay)

(event Collision|EventActorBeginOverlap
  (params (OtherActor :type Actor%20Object%20Reference)))

(event EventTick
  (params (DeltaSeconds :type Float%20%28single-precision%29))
  (bind _returnvalue (Transformation|GetActorLocation))
  (bind _direction (Variables|Default|GetDirection))
  (Transformation|SetActorLocation (Math|Vector|MakeVector (+ (* DeltaSeconds (.x _direction)) (.x _returnvalue)) (+ (* DeltaSeconds (.y _direction)) (.y _returnvalue)) (+ (* DeltaSeconds (.z _direction)) (.z _returnvalue))) false false))

(fn ConstructionScript)

(fn SetDirection
  (params (Direction :type Vector))
  (Variables|Default|SetDirection Direction))