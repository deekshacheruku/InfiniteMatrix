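; BP_Tunnel is a tunnel segment with a spinning holed wall, chained through TunnelSpawner for an endless obstacle course.
; Passing the trigger adds score, spawns the next tunnel and destroys this one.
; Hitting the wall costs BP_Player health and score, updates the UI, and shows restart at zero health.
; Externally callable functions randomize the wall mesh and roll, and spawn health packs or enemies inside the tunnel at roughly even odds.
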(event OnComponentBeginOverlap(TriggerZone)
  (params (OverlappedComponent :type Primitive%20Component%20Object%20Reference) (OtherActor :type Actor%20Object%20Reference) (OtherComp :type Primitive%20Component%20Object%20Reference) (OtherBodyIndex :type Integer) (bFromSweep :type Boolean) (SweepResult :type Hit%20Result%20Structure%20%28by%20ref%29))
  (bind _asbp_player (Utilities|Casting|CastToBP_Player OtherActor))
  (Default|IncrementScore _asbp_player)
  (Default|SpawnTunnelatSpawnPoint (Variables|Default|GetTunnelSpawner))
  (Actor|DestroyActor))

(event OnComponentBeginOverlap(WallMesh)
  (params (OverlappedComponent :type Primitive%20Component%20Object%20Reference) (OtherActor :type Actor%20Object%20Reference) (OtherComp :type Primitive%20Component%20Object%20Reference) (OtherBodyIndex :type Integer) (bFromSweep :type Boolean) (SweepResult :type Hit%20Result%20Structure%20%28by%20ref%29))
  (bind _asbp_player (Utilities|Casting|CastToBP_Player OtherActor))
  (bind _output_get (Variables|/Game/InfiniteMatrix/Blueprints/BP_Player.BP_Player_C|SetHealth _asbp_player (- (Variables|/Game/InfiniteMatrix/Blueprints/BP_Player.BP_Player_C|GetHealth _asbp_player) 10)))
  (Default|UpdateProgressBar (Variables|/Game/InfiniteMatrix/Blueprints/BP_Player.BP_Player_C|Getui _asbp_player))
  (Default|UpdateHealthScore (Variables|/Game/InfiniteMatrix/Blueprints/BP_Player.BP_Player_C|Getui _asbp_player))
  (Default|DecrementScore _asbp_player)
  (if (not (> _output_get 0))
    (Variables|/Game/InfiniteMatrix/Blueprints/BP_Player.BP_Player_C|SetIsDead _asbp_player true)
    (Default|DisplayRestart _asbp_player)))

(event EventBeginPlay)

(event EventTick
  (params (DeltaSeconds :type Float%20%28single-precision%29))
  (Transformation|AddLocalRotation (Variables|Default|GetWallMesh) (Math|Rotator|MakeRotator (* DeltaSeconds (Variables|Default|GetRotateSpeed)) 0.0 0.0) false false))

(fn ConstructionScript)

(fn RandomizeWall
  (Components|StaticMesh|SetStaticMesh (Variables|Default|GetWallMesh) (Utilities|Select :Index (Math|Random|RandomIntegerinRange 0 3) :Option%200 "/Game/InfiniteMatrix/Meshes/SM_Hole_01.SM_Hole_01" :Option%201 "/Game/InfiniteMatrix/Meshes/SM_Hole_02.SM_Hole_02" :Option%202 "/Game/InfiniteMatrix/Meshes/SM_Hole_03.SM_Hole_03" :Option%203 "/Game/InfiniteMatrix/Meshes/SM_Hole_04.SM_Hole_04"))
  (Transformation|AddLocalRotation (Variables|Default|GetWallMesh) (Math|Rotator|MakeRotator (Math|Random|RandomFloatinRange 0.0 3.6e+02) 0.0 0.0) false false))

(fn RandamizeHealthPack
  (params (SpawnLoc :type Vector))
  (if (== (Math|Integer|%(Integer) (Math|Random|RandomIntegerinRange 0 100) 2) 1)
    (bind _random_loc (CallFunction|GetLocationinTunnel 0.0 SpawnLoc))
    (bind _returnvalue (Game|SpawnActorfromClass "/Game/InfiniteMatrix/Blueprints/BP_HealthPack.BP_HealthPack_C" (Math|Transform|MakeTransform _random_loc "0.000000,100.000000, 0" "1,1,1") "Undefined" 0 0))
    (Variables|Default|SetHealthPack _returnvalue)))

(fn GetLocationinTunnel
  (params (offset :type Float%20%28single-precision%29) (SpawnLocation :type Vector))
  (return (Math|Vector|MakeVector (Math|Random|RandomFloatinRange (+ (.x SpawnLocation) 7.5e+02 offset) (+ (.x SpawnLocation) 2.2e+03)) (Math|Random|RandomFloatinRange (- (.y SpawnLocation) 2e+02) (+ (.y SpawnLocation) 2e+02)) (Math|Random|RandomFloatinRange (- (.z SpawnLocation) 2e+02) (+ (.z SpawnLocation) 2e+02)))))

(fn RandamizeEnemy
  (params (SpawnLoc :type Vector) (offset :type Float%20%28single-precision%29))
  (if (== (Math|Integer|%(Integer) (Math|Random|RandomIntegerinRange 0 100) 2) 1)
    (bind _random_loc (CallFunction|GetLocationinTunnel offset SpawnLoc))
    (bind _returnvalue (Game|SpawnActorfromClass "/Game/InfiniteMatrix/Blueprints/BP_Enemy.BP_Enemy_C" (Math|Conversions|ToTransform(Vector) _random_loc) "Undefined" 0 0))
    (Variables|Default|SetEnemy _returnvalue)))